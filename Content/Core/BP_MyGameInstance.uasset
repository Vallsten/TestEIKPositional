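; Game instance that creates or joins an Epic Online Services lobby through EIK, using a fixed lobby ID, and starts voice chat.
; The host server-travels to the game map as a listen server, and both paths switch to game-only input.
; Voice setup chains async callbacks from initialize through connect, login with a random name and room token to joining a team room.
; A helper returns the Epic display name or a not-logged-in fallback.
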(event `JoinLobby`
  (bind _foundresult (`EIK_FindSessionByID_AsyncFunction.FindEIKSessionByID` "Test8")
    (:`OnSuccess`
      (`EIK_JoinSession_AsyncFunction.JoinEIKSessions` "GameSession" _foundresult
        (:`OnSuccess`
          (`self.SetGameMode` false)
          (`self.PeterVoiceChat`))))))

(event `CreateLobby`
  ; Create Lobby
  (`EIK_CreateLobby_AsyncFunction.CreateEIKLobby` :`SessionName` "GameSession" :`NumberOfPublicConnections` 5 :`ExtraSettings` (make `CreateLobbySettings` false true 0 true true "RE_NoSelection" false true "" true true "Test8")
    (:`OnSuccess`
      (`self.SetGameMode` false)
      (`KismetSystemLibrary.ExecuteConsoleCommand` "servertravel ThirdPersonMapGame?listen" null)
      (`self.PeterVoiceChat`))
    (:`OnFail`
      (`KismetSystemLibrary.PrintString` "Fail to create lobby" true true (struct :`G` 0.66 :`B` 1.0 :`A` 1.0) 5.0))))

(event `PeterVoiceChat`
  ; Connect to Voice Chat
  (bind _returnvalue (`EVIK_Functions.InitializeEOSVoiceChat`))
  (if _returnvalue
    (`EVIK_Functions.ConnectVoiceChat` (delegate `ConnectToEOSVoiceChat_Result`))
    (else
      (`KismetSystemLibrary.PrintString` "Fail initialize voice chat"))))

(event `ConnectToEOSVoiceChat_Result`
  (params (bWasSuccess :type Boolean) (Result :type "EEVIKResultCodes Enum" :default "Success"))
  ; Connect to Voice Chat
  (if bWasSuccess
    (`EVIK_Functions.LoginEOSVoiceChat` (`KismetStringLibrary.Concat_StrStr` "Playername" (`KismetStringLibrary.Conv_IntToString` (`KismetMathLibrary.RandomInteger` 100))) (delegate `LoginToEOSVoiceChat_Result`))
    (else
      (`KismetSystemLibrary.PrintString` "Fail connect voice chat"))))

(event `LoginToEOSVoiceChat_Result`
  (params (bWasSuccess :type Boolean) (Result :type "EEVIKResultCodes Enum" :default "Success"))
  ; Connect to Voice Chat
  (if bWasSuccess
    (`EVIK_Functions.EOSRoomToken` "Team1" (`EVIK_Functions.LoggedInUser`) "10.0.0.1" (delegate `GetEOSVoiceRoomTokenMain_Result`))
    (else
      (`KismetSystemLibrary.PrintString` "Login to EOS Voice Chat Failed"))))

(event `GetEOSVoiceRoomTokenMain_Result`
  (params (bWasSuccess :type Boolean) (RoomData :type String))
  ; Connect to Voice Chat
  (if bWasSuccess
    (`EVIK_Functions.JoinEOSRoom` "Team1" RoomData false (delegate `JoinEOSVoiceRoomMain_Result`))
    (else
      (`KismetSystemLibrary.PrintString` "Fail get room token"))))

(event `JoinEOSVoiceRoomMain_Result`
  (params (bWasSuccess :type Boolean) (Result :type "EEVIKResultCodes Enum" :default "Success"))
  ; Connect to Voice Chat
  (if bWasSuccess
    (`KismetSystemLibrary.PrintString` "Join main voice room success")
    (else
      (`KismetSystemLibrary.PrintString` "Join main voice room failed"))))

(fn `GetPlayerNameBP`
  (returns (PlayerName :type Text))
  (bind _returnvalue (`EIK_BlueprintFunctions.GetEpicAccountId`))
  (bind _eik_epicaccountid (make `EIK_EpicAccountId` _returnvalue))
  (bind _outuserinfo (`EIK_UserInfoSubsystem.EIK_UserInfo_CopyUserInfo` _eik_epicaccountid _eik_epicaccountid))
  (bind (_userid _country _displayname) (break `EIK_UserInfo` _outuserinfo))
  (if (`KismetStringLibrary.NotEqual_StrStr` _displayname)
    (return (`KismetTextLibrary.Conv_StringToText` _displayname))
    (else
      (return "Not Logged In"))))

(fn `SetGameMode`
  (params (IsUIOnly :type Boolean))
  (bind _returnvalue (`GameplayStatics.GetPlayerController` 0))
  (if IsUIOnly
    (`WidgetBlueprintLibrary.SetInputMode_UIOnlyEx` _returnvalue null)
    (else
      (`WidgetBlueprintLibrary.SetInputMode_GameOnly` _returnvalue)))
  (set `PlayerController.bShowMouseCursor` (`local.IsUIOnly`) _returnvalue))